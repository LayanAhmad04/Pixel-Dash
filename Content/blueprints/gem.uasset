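; Gem pickup actor that serves as the level's win trigger.
; When its box component is overlapped by the referenced player character, it stops the timer held on that player's HUD, shows a Winscreen widget and destroys itself.
; All logic sits in that one overlap event; BeginPlay, Tick and the construction script add nothing, and the file does not set the player reference itself.
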(event `self.Box.OnComponentBeginOverlap`
  (params (OverlappedComponent :type "PrimitiveComponent Object Reference") (OtherActor :type "Actor Object Reference") (OtherComp :type "PrimitiveComponent Object Reference") (OtherBodyIndex :type Integer) (bFromSweep :type Boolean) (SweepResult :type "HitResult Structure (by ref)"))
  (bind _playercharacterref (`self.playercharacterref`))
  (if (== OtherActor _playercharacterref)
    (`KismetSystemLibrary.K2_ClearAndInvalidateTimerHandle` (`/Game/UI/playershud.timerevent` (`/Game/blueprints/2dplayercharacter.playerhud` _playercharacterref)))
    (bind _returnvalue (`|CreateWidget` "/Game/UI/winscreen.winscreen_C"))
    (`UserWidget.AddToViewport` _returnvalue 0)
    (`self.K2_DestroyActor`)))

(fn `UserConstructionScript`
  (`parent.UserConstructionScript`))